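; Player character for WinterCommotion that applies the arcade game mode's per-level options on spawn and handles death and victory.
; BeginPlay caches game framework references, sets movement, camera and input/blizzard values, and optionally adds a point light for dark levels.
; Health-component death ragdolls the mesh, with the actor following it on Tick; kill volumes deal lethal damage.
; The PlayerState's win event disables input, plays a victory animation, then shows the win screen.
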(event `self.ReceiveBeginPlay`
  (`|ExecutionSequence`
    (:`then_0`
      (`self.Casts`))
    (:`then_1`
      (`self.Binds`))
    (:`then_2`
      (set `self.S Level Options` (`/Game/_WinterCommotion/Core/GameMods/GM_Arcade.S Levels Option` (`self.As GM Arcade`))))
    (:`then_3`
      (`self.SetLevelOptions`))
    (:`then_4`
      (`self.LevelDarker`))))

(event `self.BP_HealthComponent.OnOwnerDied`
  (bind _mesh (`self.Mesh`))
  (set `self.bIsDead` true)
  (`GameplayStatics.SpawnEmitterAtLocation` "/Game/_WinterCommotion/VFX/Realistic_Starter_VFX_Pack_Vol2/Particles/Destruction/P_Destruction_Ceramic.P_Destruction_Ceramic" (`self.K2_GetActorLocation`))
  (`self.DisableInput` (`GameplayStatics.GetPlayerController` 0))
  (set `SpringArmComponent.bDoCollisionTest` false (`self.SpringArm`))
  (`PrimitiveComponent.SetCollisionEnabled` (`self.CapsuleComponent`) "NoCollision")
  (`PrimitiveComponent.SetCollisionEnabled` _mesh "QueryAndPhysics")
  (`PrimitiveComponent.SetSimulatePhysics` _mesh true)
  (`SkeletalMeshComponent.OverrideAnimationData` (`self.Mesh`) "/Game/_WinterCommotion/Character/Anims/Falling_Flat_Impact.Falling_Flat_Impact" false false 0.0 1.0))

(event `OnPlayerWin`
  (`self.DisableInput` (`GameplayStatics.GetPlayerController` 0))
  (set `SpringArmComponent.bDoCollisionTest` false (`self.SpringArm`))
  (`PrimitiveComponent.SetCollisionEnabled` (`self.CapsuleComponent`) "NoCollision")
  (`PrimitiveComponent.SetCollisionEnabled` (`self.Mesh`) "QueryAndPhysics")
  (`SkeletalMeshComponent.OverrideAnimationData` (`self.Mesh`) "/Game/_WinterCommotion/Character/Anims/Victory_Idle.Victory_Idle" false true 0.0 1.0)
  (`KismetSystemLibrary.Delay` 1.5)
  (`self.ShowWinScreen`))

(event `self.ReceiveTick`
  (params (DeltaSeconds :type "Float (single-precision)"))
  (if (`self.bIsDead`)
    (`self.K2_SetActorLocation` (`SceneComponent.K2_GetComponentLocation` (`self.Mesh`)))))

(event `self.ReceiveActorBeginOverlap`
  (params (OtherActor :type "Actor Object Reference"))
  (bind _askill_zvolume (cast `KillZVolume` OtherActor))
  (`GameplayStatics.ApplyDamage` self (`/Game/_WinterCommotion/Blueprints/ActorComponents/BP_Health_Comp.Get_Health` (`self.BP_HealthComponent`)) null _askill_zvolume))

(fn `Binds`
  (`|ExecutionSequence`
    (:`then_0`
      (add `/Game/_WinterCommotion/Core/PlayerStates/PS_WinterCommotion.OnPlayerWin` (`self.As PS Winter Commotion`) (`|CreateDelegate` :!event `OnPlayerWin`)))))

(fn `Casts`
  (`|ExecutionSequence`
    (:`then_0`
      (bind _asps_winter_commotion (cast `/Game/_WinterCommotion/Core/PlayerStates/PS_WinterCommotion` (`GameplayStatics.GetPlayerState` 0)))
      (set `self.As PS Winter Commotion` _asps_winter_commotion))
    (:`then_1`
      (bind _asgi_winter_commotion (cast `/Game/_WinterCommotion/Core/GameInstances/GI_WinterCommotion` (`GameplayStatics.GetGameInstance`)))
      (set `self.As GI Winter Commotion` _asgi_winter_commotion))
    (:`then_2`
      (bind _asgm_arcade (cast `/Game/_WinterCommotion/Core/GameMods/GM_Arcade` (`GameplayStatics.GetGameMode`)))
      (set `self.As GM Arcade` _asgm_arcade))))

(fn `LevelDarker`
  (if (`self.Is Enable Point Light`)
    (bind _returnvalue (`AddComponent|NODE_AddPointLightComponent-0` :`RelativeTransform` (`KismetMathLibrary.MakeTransform` (100.0 0.0 0.0))))
    (`LightComponentBase.SetCastShadows` _returnvalue false)
    (`LightComponent.SetIntensity` _returnvalue 30.0)
    (`PointLightComponent.SetSourceRadius` _returnvalue 0.0)
    (`LocalLightComponent.SetAttenuationRadius` _returnvalue 1000.0)
    (`PointLightComponent.SetSoftSourceRadius` _returnvalue 0.0)))

(fn `SetLevelOptions`
  (bind ((`bIsEnablePointLight_9_E7CE83B049CCDB99BCAD0E9DFACCD2B1` _bisenablepointlight) (`Gravity_38_D0FF769943DADB0AC99792AF57C293B6` _gravity) (`BlizzradSpeed_42_01FA3EC6498A407BA35A0982C42E8EED` _blizzradspeed) (`InputDelay_44_EB0A52AE436D6817BE12EE920CD9C70F` _inputdelay) (`CameraRotator_53_0515325D460DC59DDFB8E9ADAC29AC93` _camerarotator)) (break `/Game/_WinterCommotion/Core/Structures/S_LevelOptions` (`self.S Level Options`)))
  (set `CharacterMovementComponent.MaxWalkSpeed` (`self.WalkSpeed`) (`self.CharacterMovement`))
  (set `self.Is Enable Point Light` _bisenablepointlight)
  (set `CharacterMovementComponent.GravityScale` _gravity (`self.CharacterMovement`))
  (set `self.Blizzrad Speed` _blizzradspeed)
  (set `self.Input Delay` _inputdelay)
  (`SceneComponent.K2_SetWorldRotation` (`self.Camera`) _camerarotator false false))

(fn `UserConstructionScript`)