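; Actor component that spawns the level's configured shootable actor (a snowball, by its name) at its owner's SphereComponent location.
; On BeginPlay it caches the arcade GameMode and WinterCommotion GameState, then reads ActorToShoot from level options and stores base ball damage.
; SpawnBallEvent triggers the spawn, adjusting for collisions but always spawning.
; The dispatcher binding is unconnected, and the stored damage is unused here.
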(event `self.ReceiveBeginPlay`
  (`|ExecutionSequence`
    (:`then_0`
      (`self.Casts`))
    (:`then_1`
      (`self.GetLevelOptions`))
    (:`then_2`
      (`self.Set_BallDamageVar`))))

(event `SpawnBallEvent`
  (`self.SpawnBall`))

(fn `Binds`)

(fn `Casts`
  (`|ExecutionSequence`
    (:`then_0`
      (bind _asgm_arcade (cast `/Game/_WinterCommotion/Core/GameMods/GM_Arcade` (`GameplayStatics.GetGameMode`)))
      (set `self.GM_WinterCommotion` _asgm_arcade))
    (:`then_1`
      (bind _asgs_winter_commotion (cast `/Game/_WinterCommotion/Core/GameStates/GS_WinterCommotion` (`GameplayStatics.GetGameState`)))
      (set `self.GS_WinterCommotion` _asgs_winter_commotion))))

(fn `GetLevelOptions`
  (bind _output_get (set `self.S Level Options` (`/Game/_WinterCommotion/Core/GameMods/GM_Arcade.S Levels Option` (`self.GM_WinterCommotion`))))
  (set `self.ActorToShoot` (`.ActorToShoot_64_77B44D3F496D285C863A3B8673E93838` (break `/Game/_WinterCommotion/Core/Structures/S_LevelOptions` _output_get))))

(fn `Set_BallDamageVar`
  (bind _gm_wintercommotion (`self.GM_WinterCommotion`)
    (:`then`
      (set `self.BaseBallDamage` (`/Game/_WinterCommotion/Core/GameMods/GM_Arcade.Get_BallDamage` _gm_wintercommotion)))
    (:`else`)))

(fn `SpawnBall`
  (bind _returnvalue (`Actor.GetComponentByClass` (`self.GetOwner`) "/Script/Engine.SphereComponent"))
  (`/Engine/EditorBlueprintResources/StandardMacros.IsValid` _returnvalue
    (:`Is Valid`
      (`|SpawnActorFromClass` (`self.ActorToShoot`) (`KismetMathLibrary.Conv_VectorToTransform` (`SceneComponent.K2_GetComponentLocation` _returnvalue)) "AdjustIfPossibleButAlwaysSpawn" "OverrideRootScale" null null))))