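; Actor component that starts and ends a bonus when a Player-tagged actor begins or stops overlapping its owner.
; On BeginPlay it binds to the owner's overlap events, then either fires the start or end bonus event directly or sets an optional one-shot delay timer.
; StartBonusEvent and EndBonusEvent only clear their own timer handles here, with no bonus effect implemented.
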(event `self.ReceiveBeginPlay`
  (bind _returnvalue (`self.GetOwner`))
  (add `Actor.OnActorBeginOverlap` _returnvalue (`|CreateDelegate` :!event `OnActorBeginOverlap_Event`))
  (add `Actor.OnActorEndOverlap` _returnvalue (`|CreateDelegate` :!event `OnActorEndOverlap_Event`)))

(event `OnActorBeginOverlap_Event`
  (params (OverlappedActor :type "Actor Object Reference") (OtherActor :type "Actor Object Reference"))
  (`/Engine/EditorBlueprintResources/StandardMacros.IsValid` OtherActor
    (:`Is Valid`
      (if (`Actor.ActorHasTag` OtherActor "Player")
        (if (`self.HasStartDelay?`)
          (bind _returnvalue (`KismetSystemLibrary.K2_SetTimerDelegate` (`|CreateDelegate` :!event `StartBonusEvent`) (`self.StartDelay`)))
          (set `self.StartHandler` _returnvalue)
          (else
            (`self.StartBonusEvent`)))))))

(event `OnActorEndOverlap_Event`
  (params (OverlappedActor :type "Actor Object Reference") (OtherActor :type "Actor Object Reference"))
  (`/Engine/EditorBlueprintResources/StandardMacros.IsValid` OtherActor
    (:`Is Valid`
      (if (`Actor.ActorHasTag` OtherActor "Player")
        (if (`self.HasEndDelay?`)
          (bind _returnvalue (`KismetSystemLibrary.K2_SetTimerDelegate` (`|CreateDelegate` :!event `EndBonusEvent`) (`self.EndDelay`)))
          (set `self.EndHandler` _returnvalue)
          (else
            (`self.EndBonusEvent`)))))))

(event `EndBonusEvent`
  (bind _endhandler (`self.EndHandler`))
  (if (`KismetSystemLibrary.K2_IsValidTimerHandle` _endhandler)
    (`KismetSystemLibrary.K2_ClearAndInvalidateTimerHandle` _endhandler)))

(event `StartBonusEvent`
  (bind _starthandler (`self.StartHandler`))
  (if (`KismetSystemLibrary.K2_IsValidTimerHandle` _starthandler)
    (`KismetSystemLibrary.K2_ClearAndInvalidateTimerHandle` _starthandler)))