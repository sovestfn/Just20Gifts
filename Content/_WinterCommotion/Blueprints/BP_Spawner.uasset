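; Spawner actor that fills its Box area with configured object types at BeginPlay, one randomly assigned to each grid point.
; It sizes a near-square grid from the summed ObjectCounts and computes cell positions across the Box bounds at world Z zero.
; ObjectTypes are expanded by count into a shuffled queue, then spawned by position index and stored in SpawnedActors.
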(event EventBeginPlay
  (bind _box (Variables|Default|GetBox))
  (bind (_origin _boxextent) (Collision|GetComponentBounds _box))
  (Utilities|FlowControl|Sequence
    (:then_0
      ;[1 1 1] Calc start spawn point
      (Variables|Default|SetFirstSpawnPointLocal (Math|Vector|MakeVector (- (.x _origin) (.x _boxextent)) (- (.y _origin) (.y _boxextent)) 0.0))
      (Variables|Default|SetxSize (* (.x _boxextent) 2.0))
      (Variables|Default|SetySize (* (.y _boxextent) 2.0)))
    (:then_2
      (CallFunction|GenerateGridPositions)
      (CallFunction|GenerateObjectQueue)
      (CallFunction|SpawnObjects))))

(fn ConstructionScript)

(fn GenerateGridPositions
  (bind _firstspawnpointlocal (Variables|Default|GetFirstSpawnPointLocal))
  (Utilities|FlowControl|Sequence
    (:then_0
      (for _array_element (Variables|Default|GetObjectCounts)
        (LocalVariables|SetTotalObjects (+ _array_element (LocalVariables|GetTotalObjects)))))
    (:then_1
      (Variables|Default|Setcols (Math|Float|Ceil (Math|Float|Sqrt (Math|Conversions|ToFloat(Integer) (LocalVariables|GetTotalObjects))))))
    (:then_2
      (Variables|Default|Setrows (Math|Float|Ceil (/ (LocalVariables|GetTotalObjects) (Variables|Default|Getcols)))))
    (:then_3
      (for _index (range 1 (Variables|Default|Getrows))
        (for _index_2 (range 1 (Variables|Default|Getcols))
          (bind _output_get (Variables|Default|SetYcoord (- (* _index (|({76CF2D99-43B2-0467-B6E6-55820B752820}/{C4287092-48D4-5F02-CA67-E4BCDB47F2ED}))) (|(({76CF2D99-43B2-0467-B6E6-55820B752820}/{C4287092-48D4-5F02-CA67-E4BCDB47F2ED})/2)))))
          (bind _output_get_2 (Variables|Default|SetXcoord (- (* _index_2 (|({8118D00F-4493-BE13-46B7-489B2F127CD1}/{1E1B9243-4E7D-F32B-C6CA-DD8B4327AD1F}))) (|(({8118D00F-4493-BE13-46B7-489B2F127CD1}/{1E1B9243-4E7D-F32B-C6CA-DD8B4327AD1F})/2)))))
          (Utilities|Array|Add (Variables|Default|GetpositionList%20) (Math|Vector|MakeVector (+ (.x _firstspawnpointlocal) _output_get_2) (+ (.y _firstspawnpointlocal) _output_get) 0.0)))))))

(fn GenerateObjectQueue
  (for (_array_element _array_index) (Variables|Default|GetObjectTypes)
    (for _index (range 0 (- (Utilities|Array|Get(acopy) (Variables|Default|GetObjectCounts) _array_index) 1))
      (Utilities|Array|Add (Variables|Default|GetObjectQueue%20) _array_element)
      (Utilities|Array|Shuffle (Variables|Default|GetObjectQueue%20)))))

(fn SpawnObjects
  (for (_array_element _array_index) (Variables|Default|GetpositionList%20)
    (bind _returnvalue (Game|SpawnActorfromClass (Utilities|Array|Get(acopy) (Variables|Default|GetObjectQueue%20) _array_index) (Math|Transform|MakeTransform _array_element) "AdjustIfPossibleButAlwaysSpawn" "MultiplyWithRoot" 0 0))
    (Utilities|Array|Add (Variables|Default|GetSpawnedActors%20) _returnvalue)))