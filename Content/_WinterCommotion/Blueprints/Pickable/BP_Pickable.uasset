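; BP_Pickable is a pickup actor that is collected when an actor tagged Player overlaps it.
; On overlap, after checking that player pawn 0 is valid, it calls the OnPicked dispatcher and plays a sound at its location.
; DestroyPickable then spawns a scaled-up particle effect and destroys the actor on the next tick.
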(event `self.ReceiveActorBeginOverlap`
  (params (OtherActor :type "Actor Object Reference"))
  (`/Engine/EditorBlueprintResources/StandardMacros.IsValid` (`GameplayStatics.GetPlayerPawn` 0)
    (:`Is Valid`
      (if (`self.ActorHasTag` OtherActor "Player")
        (`self.OnPicked`)
        (`GameplayStatics.PlaySoundAtLocation` (`self.Sound`) (`self.K2_GetActorLocation`) (struct) 1.0 1.0 0.0 null null null null)
        (`self.DestroyPickable`)))))

(event `DestroyPickable`
  (`GameplayStatics.SpawnEmitterAtLocation` (`self.DestroyEffect`) (`self.K2_GetActorLocation`) (struct) (2.0 2.0 2.0))
  (`KismetSystemLibrary.DelayUntilNextTick`)
  (`self.K2_DestroyActor`))

(fn `UserConstructionScript`)