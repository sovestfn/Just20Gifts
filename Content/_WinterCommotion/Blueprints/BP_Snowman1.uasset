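; Snowman enemy that turns toward the player and spawns balls when the player enters its overlap area.
; Entering fires the spawner component and starts a looping timer, paced by level options from GM_Arcade, which is cleared when the player leaves.
; A turn-to-player component runs every Tick, while a health component takes damage and destroys the actor on death.
; The construction script randomly varies the snowman's material.
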(event `self.ReceiveBeginPlay`
  (`|ExecutionSequence`
    (:`then_0`
      (bind _asgm_arcade (cast `/Game/_WinterCommotion/Core/GameMods/GM_Arcade` (`GameplayStatics.GetGameMode`)))
      (set `self.As GM Arcade` _asgm_arcade))
    (:`then_1`
      (set `self.S Level Options` (`/Game/_WinterCommotion/Core/GameMods/GM_Arcade.S Levels Option` (`self.As GM Arcade`))))))

(event `self.ReceiveActorBeginOverlap`
  (params (OtherActor :type "Actor Object Reference"))
  (if (`self.ActorHasTag` OtherActor "Player")
    (bind _returnvalue (`KismetSystemLibrary.K2_SetTimerDelegate` (`|CreateDelegate` (`self.BP_SpawnerComponent`) :!event `SpawnBall`) (`.TimeToSpawnShoot_40_92CEBD384590A0E1025A39920FB64C69` (break `/Game/_WinterCommotion/Core/Structures/S_LevelOptions` (`self.S Level Options`))) true))
    (set `self.SpawnTimerHandler` _returnvalue)
    (`/Game/_WinterCommotion/Blueprints/ActorComponents/BP_SnowballSpawner_Comp.SpawnBall` (`self.BP_SpawnerComponent`))))

(event `self.ReceiveActorEndOverlap`
  (params (OtherActor :type "Actor Object Reference"))
  (if (`self.ActorHasTag` OtherActor "Player")
    (`KismetSystemLibrary.K2_ClearAndInvalidateTimerHandle` (`self.SpawnTimerHandler`))))

(event `self.ReceiveTick`
  (params (DeltaSeconds :type "Float (single-precision)"))
  (`/Game/_WinterCommotion/Blueprints/ActorComponents/BP_TurnToPlayer_Comp.TurnToPlayer` (`self.BP_TurnToPlayerComponent`)))

(event `self.ReceiveAnyDamage`
  (params (Damage :type "Float (single-precision)") (DamageType :type "DamageType Object Reference") (InstigatedBy :type "Controller Object Reference") (DamageCauser :type "Actor Object Reference"))
  (bind _bp_health_comp (`self.BP_Health_Comp`))
  (`/Game/_WinterCommotion/Blueprints/ActorComponents/BP_Health_Comp.Set_Health` _bp_health_comp (- (`/Game/_WinterCommotion/Blueprints/ActorComponents/BP_Health_Comp.Get_Health` _bp_health_comp) Damage)))

(event `self.BP_Health_Comp.OnOwnerDied`
  (`self.K2_DestroyActor`))

(fn `Casts`
  (`|ExecutionSequence`
    (:`then_0`
      (cast `/Game/_WinterCommotion/Core/GameStates/GS_WinterCommotion` (`GameplayStatics.GetGameState`)))
    (:`then_1`
      (cast `/Game/_WinterCommotion/Core/GameMods/GM_Arcade` (`GameplayStatics.GetGameMode`)))))

(fn `UserConstructionScript`
  (locals (SnowmanMaterials :type "Array of MaterialInstance Object Reference"))
  (for _array_element (`self.MaterialSnowman`)
    (if (`KismetMathLibrary.RandomBoolWithWeight` 0.3)
      (`PrimitiveComponent.SetMaterial` (`self.Snowman`) 0 _array_element))))