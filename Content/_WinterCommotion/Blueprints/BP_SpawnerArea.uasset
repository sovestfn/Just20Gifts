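; Spawner area actor that fills its Spawner bounds at BeginPlay with the actor classes from GM_Arcade's level options.
; It divides the bounds into an X-by-Y grid, jitters a point around each cell center by a spread percentage, and spawns every listed class there.
; With CanRespawn, destruction events are bound for timed respawning; Respawn places the separate ItemForSpawn class at a random point in the box.
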(event `self.ReceiveBeginPlay`
  (`|ExecutionSequence`
    (:`then_0`
      (bind _asgm_arcade (cast `/Game/_WinterCommotion/Core/GameMods/GM_Arcade` (`GameplayStatics.GetGameMode`)))
      (bind _output_get (set `self.As GM Arcade` _asgm_arcade))
      (bind _output_get_2 (set `self.S Levels Option` (`/Game/_WinterCommotion/Core/GameMods/GM_Arcade.S Levels Option` _output_get)))
      (set `self.Actors for Spawn Area` (`.ActorsForSpawnArea_69_BF18D6314B880A875516278CBE11E162` (break `/Game/_WinterCommotion/Core/Structures/S_LevelOptions` _output_get_2))))
    (:`then_2`
      (set `self.CountOfItems` (* (`self.ItemsInRow(X)`) (`self.ItemsInСolumn(Y)`))))
    (:`then_3`
      (`self.SpawnItemInVolumeFunction`))))

(fn `CalcSpawnItemsLocation`
  (returns (SpawnLocations :type "Array of Vector Structure"))
  (locals (SpredX :type "Float (double-precision)") (SpredY :type "Float (double-precision)") (FirstSpawnPointLocal :type "Vector Structure" :default (0.0 0.0 0.0)) (SpawnLocationLocal :type "Array of Vector Structure"))
  (bind (_origin _boxextent) (`KismetSystemLibrary.GetComponentBounds` (`self.spawner`)))
  (bind (_returnvalue_x _returnvalue_y _returnvalue_z) (`KismetMathLibrary.BreakVector` (`SceneComponent.K2_GetComponentLocation` (`self.spawner`))))
  (bind _returnvalue (/ (`KismetMathLibrary.Conv_IntToDouble` (`self.SpredPercent`)) 100))
  (`|ExecutionSequence`
    (:`then_0`
      ;[1 1 1] Calc start spawn point
      (set `local.FirstSpawnPointLocal` (`KismetMathLibrary.MakeVector` (- (.x _origin) (.x _boxextent)) (- (.y _origin) (.y _boxextent))))
      ;[1 1 1] Calc spawn area for each item
      (bind _output_get (set `self.ItemAreaSideX` (/ (* (.x _boxextent) 2.0) (`self.ItemsInRow(X)`))))
      (bind _output_get_2 (set `self.ItemAreaSideY` (/ (* (.y _boxextent) 2.0) (`self.ItemsInСolumn(Y)`))))
      ;[1 1 1] Calc spred
      (set `local.SpredX` (* (/ _output_get 2.0) _returnvalue))
      (set `local.SpredY` (* _returnvalue (/ _output_get_2 2.0)))
      ;[1 1 1] Calc spawn location  for each item
      (for _index (range (`self.ItemsInRow(X)`))
        (for _index_2 (range (`self.ItemsInСolumn(Y)`))
          (bind _returnvalue_2 (+ (+ (.x (`local.FirstSpawnPointLocal`)) (* (`self.ItemAreaSideX`) _index)) (/ (`self.ItemAreaSideX`) 2.0)))
          (bind _returnvalue_3 (+ (+ (.y (`local.FirstSpawnPointLocal`)) (* (`self.ItemAreaSideY`) _index_2)) (/ (`self.ItemAreaSideY`) 2.0)))
          (`KismetArrayLibrary.Array_Add` (`local.SpawnLocationLocal`) (`KismetMathLibrary.MakeVector` (`KismetMathLibrary.RandomFloatInRange` (- _returnvalue_2 (`local.SpredX`)) (+ _returnvalue_2 (`local.SpredX`))) (`KismetMathLibrary.RandomFloatInRange` (- _returnvalue_3 (`local.SpredY`)) (+ _returnvalue_3 (`local.SpredY`))) _returnvalue_z)))))
    (:`then_1`
      (return (`local.SpawnLocationLocal`)))))

(fn `DelayBeforeRespawn`
  (params (DestroyedActor :type "Actor Object Reference"))
  (bind _returnvalue (`KismetSystemLibrary.K2_SetTimerDelegate` (`|CreateDelegate` :!event `Respawn`) (`self.RespawnTime`)))
  (set `self.TimerHadler` _returnvalue))

(fn `Respawn`
  (bind (_origin _boxextent) (`KismetSystemLibrary.GetComponentBounds` (`self.spawner`)))
  ;[1 1 1] не нравится повторяющаяся логика, но пока не знаю, как реализовать по другому
  (bind _returnvalue (`|SpawnActorFromClass` (`self.ItemForSpawn`) (`KismetMathLibrary.MakeTransform` (`KismetMathLibrary.RandomPointInBoundingBox` _origin _boxextent)) "AdjustIfPossibleButAlwaysSpawn" "MultiplyWithRoot" null null))
  (`/Engine/EditorBlueprintResources/StandardMacros.IsValid` _returnvalue
    (:`Is Valid`
      (add `self.OnDestroyed` _returnvalue (`|CreateDelegate` :!event `DelayBeforeRespawn`))
      (`KismetSystemLibrary.K2_ClearAndInvalidateTimerHandle` (`self.TimerHadler`)))))

(fn `SpawnItemInVolumeFunction`
  (bind _spawnlocations (`self.CalcSpawnItemsLocation`))
  (for _array_element _spawnlocations
    (for _array_element_2 (`self.Actors for Spawn Area`)
      (bind _returnvalue (`|SpawnActorFromClass` _array_element_2 (`KismetMathLibrary.MakeTransform` _array_element) "AdjustIfPossibleButAlwaysSpawn" "MultiplyWithRoot" null null))
      (if (`self.CanRespawn?`)
        (`/Engine/EditorBlueprintResources/StandardMacros.IsValid` _returnvalue
          (:`Is Valid`
            (add `self.OnDestroyed` _returnvalue (`|CreateDelegate` :!event `DelayBeforeRespawn`))))))))

(fn `UserConstructionScript`)