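; GM_Tutorial is the tutorial game mode, which ends the game when the player dies.
; On BeginPlay it caches the game state, player character and game instance, then binds to the character's health component death event.
; EndGame and RestartGame forward to GS_WinterCommotion.
; It also holds a BallDamage value with a getter and setter.
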(event `self.ReceiveBeginPlay`
  (`|ExecutionSequence`
    (:`then_0`
      (`self.Casts`))
    (:`then_1`
      (`self.Binds`))
    (:`then_2`
      (`self.Set_BallDamage` (`self.BallDamage`)))))

(event `OnPlayerDied`
  (`self.EndGame`))

(event `RestartGame`
  (bind _gs_wintercommotion (`self.GS_WinterCommotion`)
    (:`then`
      (`/Game/_WinterCommotion/Core/GameStates/GS_WinterCommotion.RestartGame` _gs_wintercommotion))
    (:`else`)))

(event `EndGame`
  (bind _gs_wintercommotion (`self.GS_WinterCommotion`)
    (:`then`
      (`/Game/_WinterCommotion/Core/GameStates/GS_WinterCommotion.EndGame` _gs_wintercommotion))
    (:`else`)))

(fn `Binds`
  (`|ExecutionSequence`
    (:`then_0`
      (add `/Game/_WinterCommotion/Blueprints/ActorComponents/BP_Health_Comp.OnOwnerDied` (`/Game/_WinterCommotion/Character/BP_AJ_Character.BP_HealthComponent` (`self.BP_AJ_Character`)) (`|CreateDelegate` :!event `OnPlayerDied`)))))

(fn `Casts`
  (`|ExecutionSequence`
    (:`then_0`
      (bind _asgs_winter_commotion (cast `/Game/_WinterCommotion/Core/GameStates/GS_WinterCommotion` (`GameplayStatics.GetGameState`)))
      (set `self.GS_WinterCommotion` _asgs_winter_commotion))
    (:`then_1`
      (bind _asbp_aj_character (cast `/Game/_WinterCommotion/Character/BP_AJ_Character` (`GameplayStatics.GetPlayerPawn` 0)))
      (set `self.BP_AJ_Character` _asbp_aj_character))
    (:`then_2`
      (bind _asgi_winter_commotion (cast `/Game/_WinterCommotion/Core/GameInstances/GI_WinterCommotion` (`GameplayStatics.GetGameInstance`)))
      (set `self.GI_WinterCommotion` _asgi_winter_commotion))))

(fn `Get_BallDamage`
  (returns (BallDamage :type "Float (double-precision)"))
  (return (`self.BallDamage`)))

(fn `Set_BallDamage`
  (params (BallDamage :type "Float (double-precision)"))
  (set `self.BallDamage` BallDamage))

(fn `UserConstructionScript`)