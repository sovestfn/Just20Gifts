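; Arcade game mode for WinterCommotion that runs level setup, win or death handling, and level progression.
; BeginPlay caches core framework objects, binds win and death events, copies level options from the game instance, blacks out directional light for dark levels, and starts a looping autosave timer.
; Win or death ends the game through the game state and clears that timer.
; An index map of DT_LevelOptions rows advances the saved level to the next row.
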(event `self.ReceiveBeginPlay`
  (`|ExecutionSequence`
    (:`then_0`
      (`self.Casts`))
    (:`then_1`
      (`self.Binds`))
    (:`then_2`
      (`self.Set_BallDamage` (`self.BallDamage`)))
    (:`then_3`
      (`self.MakeDTMap`))
    (:`then_4`
      (`self.SetLevelOptions`))
    (:`then_5`
      (`self.LevelDarker`))
    (:`then_7`
      (bind _returnvalue (`KismetSystemLibrary.K2_SetTimerDelegate` (`|CreateDelegate` :!event `SaveGame`) 3.0 true))
      (set `self.SaveGameHandler` _returnvalue))))

(event `OnPlayerDied`
  (`self.EndGame`))

(event `OnPlayerWin`
  (`self.EndGame`))

(event `RestartGame`
  (bind _gs_wintercommotion (`self.GS_WinterCommotion`)
    (:`then`
      (`/Game/_WinterCommotion/Core/GameStates/GS_WinterCommotion.RestartGame` _gs_wintercommotion))
    (:`else`)))

(event `EndGame`
  (bind _gs_wintercommotion (`self.GS_WinterCommotion`)
    (:`then`
      (`/Game/_WinterCommotion/Core/GameStates/GS_WinterCommotion.EndGame` _gs_wintercommotion)
      (`KismetSystemLibrary.K2_ClearAndInvalidateTimerHandle` (`self.SaveGameHandler`)))
    (:`else`)))

(event `SaveGame`
  (message `/Game/_WinterCommotion/Core/Interfaces/BPI_SaveGame.SaveGame` (`self.GI_WinterCommotion`)))

(event `OnNextLevel_Event`
  (`self.ChangeLevel`))

(fn `Binds`
  (`|ExecutionSequence`
    (:`then_0`
      (add `/Game/_WinterCommotion/Core/PlayerStates/PS_WinterCommotion.OnPlayerWin` (`self.PS_WinterCommotion`) (`|CreateDelegate` :!event `OnPlayerWin`)))
    (:`then_1`
      (add `/Game/_WinterCommotion/Blueprints/ActorComponents/BP_Health_Comp.OnOwnerDied` (`/Game/_WinterCommotion/Character/BP_AJ_Character.BP_HealthComponent` (`self.BP_AJ_Character`)) (`|CreateDelegate` :!event `OnPlayerDied`)))))

(fn `Casts`
  (`|ExecutionSequence`
    (:`then_0`
      (bind _asgs_winter_commotion (cast `/Game/_WinterCommotion/Core/GameStates/GS_WinterCommotion` (`GameplayStatics.GetGameState`)))
      (set `self.GS_WinterCommotion` _asgs_winter_commotion))
    (:`then_1`
      (bind _asbp_aj_character (cast `/Game/_WinterCommotion/Character/BP_AJ_Character` (`GameplayStatics.GetPlayerPawn` 0)))
      (set `self.BP_AJ_Character` _asbp_aj_character))
    (:`then_2`
      (bind _asgi_winter_commotion (cast `/Game/_WinterCommotion/Core/GameInstances/GI_WinterCommotion` (`GameplayStatics.GetGameInstance`)))
      (set `self.GI_WinterCommotion` _asgi_winter_commotion))
    (:`then_3`
      (bind _asps_winter_commotion (cast `/Game/_WinterCommotion/Core/PlayerStates/PS_WinterCommotion` (`GameplayStatics.GetPlayerState` 0)))
      (set `self.PS_WinterCommotion` _asps_winter_commotion))
    (:`then_4`
      (bind _aspc_winter_commotion_controller (cast `/Game/_WinterCommotion/Core/PlayerController/PC_WinterCommotionController` (`GameplayStatics.GetPlayerController` 0)))
      (set `self.As PC Winter Commotion Controller` _aspc_winter_commotion_controller))))

(fn `ChangeLevel`
  (bind _gi_wintercommotion (`self.GI_WinterCommotion`))
  (bind (_value _returnvalue) (`BlueprintMapLibrary.Map_Find` (`self.DataTableIdexedRows`) (+ (`KismetArrayLibrary.Array_Find` (`self.DTLevelRowNames`) (`/Game/_WinterCommotion/Core/GameInstances/GI_WinterCommotion.SavedLevel` (`self.GI_WinterCommotion`))) 1)))
  (bind _output_get (set `self.bIsNextLevelExist` _returnvalue))
  (if _output_get
    (bind _output_get_2 (set `/Game/_WinterCommotion/Core/GameInstances/GI_WinterCommotion.SavedLevel` _value _gi_wintercommotion))
    (message `/Game/_WinterCommotion/Core/Interfaces/BPI_LevelsSettings.CurrentLevelName` _gi_wintercommotion _output_get_2)))

(fn `Get_BallDamage`
  (returns (BallDamage :type "Float (double-precision)"))
  (return (`self.BallDamage`)))

(fn `LevelDarker`
  (bind ((`bIsDarkness_7_7CFA910B4B070B7C437E9C9D43645858` _bisdarkness) (`bIsEnablePointLight_9_E7CE83B049CCDB99BCAD0E9DFACCD2B1` _bisenablepointlight)) (break `/Game/_WinterCommotion/Core/Structures/S_LevelOptions` (`self.S Levels Option`)))
  (if (and _bisdarkness _bisenablepointlight)
    (bind _returnvalue (`GameplayStatics.GetActorOfClass` "/Script/Engine.DirectionalLight"))
    (`LightComponent.SetIntensity` _returnvalue 0.0)))

(fn `MakeDTMap`
  (bind _outrownames (`DataTableFunctionLibrary.GetDataTableRowNames` "/Game/_WinterCommotion/Core/DataTables/DT_LevelOptions.DT_LevelOptions"))
  (bind _output_get (set `self.DTLevelRowNames` _outrownames))
  (for (_array_element _array_index) _output_get
    (`BlueprintMapLibrary.Map_Add` (`self.DataTableIdexedRows`) _array_index _array_element)))

(fn `Set_BallDamage`
  (params (BallDamage :type "Float (double-precision)"))
  (set `self.BallDamage` BallDamage))

(fn `SetLevelOptions`
  (set `self.S Levels Option` (`/Game/_WinterCommotion/Core/GameInstances/GI_WinterCommotion.LevelsOptions` (`self.GI_WinterCommotion`))))

(fn `UserConstructionScript`)